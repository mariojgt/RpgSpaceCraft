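; Base machine actor for the Space Factory game that can be carried, dropped and docked into machine slots.
; Its sphere overlap registers or clears it as the overlapping machine on any actor with a BPC_SpaceFactory component.
; ToogleCarryMachine either disables physics and socket-attaches it to the given parent, notifying its current slot, or drops it with physics enabled.
; A drop overlapping a BP_MachineSlot attaches it there, disables physics and stores that slot.
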(event OnComponentBeginOverlap(Sphere)
  (params (OverlappedComponent :type Primitive%20Component%20Object%20Reference) (OtherActor :type Actor%20Object%20Reference) (OtherComp :type Primitive%20Component%20Object%20Reference) (OtherBodyIndex :type Integer) (bFromSweep :type Boolean) (SweepResult :type Hit%20Result%20Structure%20%28by%20ref%29))
  (bind _returnvalue (Actor|GetComponentbyClass OtherActor "/Game/SpaceFactory/BPC_SpaceFactory.BPC_SpaceFactory_C"))
  ;[1 1 1] On player actoer enter or get out
  (Utilities|IsValid _returnvalue
    (:Is%20Valid
      (Variables|/Game/SpaceFactory/BPC_SpaceFactory.BPC_SpaceFactory_C|SetOverlapingMachine _returnvalue self))))

(event OnComponentEndOverlap(Sphere)
  (params (OverlappedComponent :type Primitive%20Component%20Object%20Reference) (OtherActor :type Actor%20Object%20Reference) (OtherComp :type Primitive%20Component%20Object%20Reference) (OtherBodyIndex :type Integer))
  (bind _returnvalue (Actor|GetComponentbyClass OtherActor "/Game/SpaceFactory/BPC_SpaceFactory.BPC_SpaceFactory_C"))
  ;[1 1 1] On player actoer enter or get out
  (Utilities|IsValid _returnvalue
    (:Is%20Valid
      (Variables|/Game/SpaceFactory/BPC_SpaceFactory.BPC_SpaceFactory_C|SetOverlapingMachine _returnvalue 0))))

(event Custom|ToogleCarryMachine
  (params (Parent :type Scene%20Component%20Object%20Reference))
  (bind _sphere (Variables|Default|GetSphere))
  (bind _overlappingactors (Collision|GetOverlappingActors _sphere "/Game/SpaceFactory/Blueprints/MachinesConnector/BP_MachineSlot.BP_MachineSlot_C" :!class /Script/Engine.PrimitiveComponent))
  (bind _output (Utilities|Array|Get(acopy) _overlappingactors))
  (if (Variables|Default|GetisCarring)
    ;[1 1 1] ItemDrop
    (Physics|SetSimulatePhysics (Variables|Default|GetStaticMesh) true)
    (Transformation|DetachFromActor self "KeepWorld" "KeepWorld" "KeepWorld")
    (Variables|Default|SetisCarring false)
    ;[1 1 1] If touch a machine Slot  them attack to that actor
    (Utilities|IsValid _output
      (:Is%20Valid
        (bind _asbp_machine_slot (Utilities|Casting|CastToBP_MachineSlot _output))
        (Default|AttachMachine _asbp_machine_slot self)
        (Physics|SetSimulatePhysics (Variables|Default|GetStaticMesh) false)
        (Variables|Default|SetCUrrentMachineSlot _asbp_machine_slot)))
    (else
      ;[1 1 1] ItemCarry
      (Physics|SetSimulatePhysics (Variables|Default|GetStaticMesh) false)
      (Transformation|AttachComponentToComponent self Parent (Variables|Default|GetCarringSocketName) "SnapToTarget" "SnapToTarget" "SnapToTarget" false)
      (Variables|Default|SetisCarring true)
      ;[1 1 1] Tell the socket is detach
      (Utilities|IsValid (Variables|Default|GetCUrrentMachineSlot)
        (:Is%20Valid
          (Default|DeatchMachineSlot (Variables|Default|GetCUrrentMachineSlot)))))))

(event EventBeginPlay)

(event Collision|EventActorBeginOverlap
  (params (OtherActor :type Actor%20Object%20Reference)))

(fn ConstructionScript)