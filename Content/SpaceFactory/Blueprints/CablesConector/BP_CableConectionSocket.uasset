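; Cable connection socket actor that players link to another socket with a spawned BP_Cable.
; Its trigger registers it as OverlapedSocket on the overlapping actor's BPC_SpaceFactory component.
; StartConnection attaches the cable end to a temporary actor; MakeConection cross-references both sockets, then recolors the cable or disconnects it if beyond max length.
; DisconnectCable destroys cables and propagates to the other socket; IsConnected's RepNotify swaps the socket material.
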(event OnComponentBeginOverlap(CollisonTrigger)
  (params (OverlappedComponent :type Primitive%20Component%20Object%20Reference) (OtherActor :type Actor%20Object%20Reference) (OtherComp :type Primitive%20Component%20Object%20Reference) (OtherBodyIndex :type Integer) (bFromSweep :type Boolean) (SweepResult :type Hit%20Result%20Structure%20%28by%20ref%29))
  (bind _returnvalue (Actor|GetComponentbyClass OtherActor "/Game/SpaceFactory/BPC_SpaceFactory.BPC_SpaceFactory_C"))
  ;[1 1 1] WHen the player overlay this actor we set to the varaible and if the player press
  (Utilities|IsValid _returnvalue
    (:Is%20Valid
      (Variables|/Game/SpaceFactory/BPC_SpaceFactory.BPC_SpaceFactory_C|SetOverlapedSocket _returnvalue self))))

(event OnComponentEndOverlap(CollisonTrigger)
  (params (OverlappedComponent :type Primitive%20Component%20Object%20Reference) (OtherActor :type Actor%20Object%20Reference) (OtherComp :type Primitive%20Component%20Object%20Reference) (OtherBodyIndex :type Integer))
  (bind _returnvalue (Actor|GetComponentbyClass OtherActor "/Game/SpaceFactory/BPC_SpaceFactory.BPC_SpaceFactory_C"))
  ;[1 1 1] when the actor get out
  (Utilities|IsValid _returnvalue
    (:Is%20Valid
      (Variables|/Game/SpaceFactory/BPC_SpaceFactory.BPC_SpaceFactory_C|SetOverlapedSocket _returnvalue 0))))

(event Custom|StartConnection
  (params (TempActor :type Actor%20Object%20Reference))
  ;[0 1 0.2159] Start the conection
  (if (not (Variables|Default|GetisConnected))
    ;;[1 1 1] Spawn the cable and connecto to the start socket
    (bind _returnvalue (Game|SpawnActorfromClass "/Game/SpaceFactory/Blueprints/CablesConector/BP_Cable.BP_Cable_C" (Transformation|GetActorTransform self) "Undefined" 0 0))
    (bind _output_get (Variables|Default|SetConectionCable _returnvalue))
    ;;[1 1 1] Temp attach teh cable to the player
    (Class|CableComponent|SetAttachEndto (Variables|/Game/SpaceFactory/Blueprints/CablesConector/BP_Cable.BP_Cable_C|GetCable _output_get) TempActor "None" "None")
    ;;[1 1 1] Change the cable material to temporary
    (Rendering|Material|SetMaterial (Variables|/Game/SpaceFactory/Blueprints/CablesConector/BP_Cable.BP_Cable_C|GetCable _output_get) 0 "/Game/SpaceFactory/Materials/M_InstanceCableMaterialNotConnected.M_InstanceCableMaterialNotConnected")))

(event Custom|MakeConection
  (params (OtherEndConection :type BP%20Cable%20Conection%20Socket%20Object%20Reference))
  (bind _conectioncable (Variables|Default|GetConectionCable))
  ;[1 1 1] Make the conection with the other socket
  (bind _output_get (Variables|Default|SetOtherEndConection OtherEndConection))
  ;;[1 1 1] Set the other end conecttion to self reference
  (Variables|BP_CableConectionSocket_C|SetOtherEndConection _output_get self)
  (Variables|Default|SetisConnected true)
  (Utilities|IsValid (Variables|Default|GetConectionCable)
    (:Is%20Valid
      (if (> (Transformation|GetDistanceTo (Components|GetOwner (Class|CableComponent|GetAttachedComponent (Variables|/Game/SpaceFactory/Blueprints/CablesConector/BP_Cable.BP_Cable_C|GetCable _conectioncable)))) (Variables|/Game/SpaceFactory/Blueprints/CablesConector/BP_Cable.BP_Cable_C|GetMaxLenght _conectioncable))
        (CallFunction|DisconnectCable)
        (else
          (Rendering|Material|SetMaterial (Variables|/Game/SpaceFactory/Blueprints/CablesConector/BP_Cable.BP_Cable_C|GetCable (Variables|Default|GetConectionCable)) 0 "/Game/SpaceFactory/Materials/M_CableConnected.M_CableConnected"))))))

(event Custom|DisconnectCable
  (bind _otherendconection (Variables|Default|GetOtherEndConection))
  (bind _conectioncable (Variables|Default|GetConectionCable))
  (bind _otherendconection_2 (Variables|Default|GetOtherEndConection))
  (bind _conectioncable_2 (Variables|BP_CableConectionSocket_C|GetConectionCable _otherendconection_2))
  ;[1 0.1342 0.0245] Disconect the cable and the other end
  ;;[1 1 1] If the cable is connect we disconect the cables
  (if (Variables|Default|GetisConnected)
    (Variables|Default|SetisConnected false)
    (Utilities|FlowControl|Sequence
      (:then_0
        (Utilities|IsValid _conectioncable
          (:Is%20Valid
            (Actor|DestroyActor _conectioncable))))
      (:then_1
        (Utilities|IsValid _conectioncable_2
          (:Is%20Valid
            (Actor|DestroyActor _conectioncable_2))))
      (:then_2
        ;;[1 1 1] Call this event on the other cable end socket
        (Utilities|IsValid _otherendconection
          (:Is%20Valid
            (CallFunction|DisconnectCable _otherendconection)))))))

(event EventBeginPlay)

(event Collision|EventActorBeginOverlap
  (params (OtherActor :type Actor%20Object%20Reference)))

(event EventTick
  (params (DeltaSeconds :type Float%20%28single-precision%29)))

(fn ConstructionScript)

(fn OnRepIsConnected
  (if (Variables|Default|GetisConnected)
    (Rendering|Material|SetMaterial (Variables|Default|GetStaticMesh) 0 "/Game/SpaceFactory/Materials/M_CableConnected.M_CableConnected")
    (else
      (Rendering|Material|SetMaterial (Variables|Default|GetStaticMesh) 0 "/Game/SpaceFactory/Materials/M_InstanceCableMaterialNotConnected.M_InstanceCableMaterialNotConnected"))))