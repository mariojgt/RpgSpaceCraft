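; Player-interaction component for Space Factory that handles cable connections between sockets, machine carrying and mouse-mode toggling.
; Interacting starts a cable at the overlapped socket, then attaches its end to the next socket and links both ways.
; Interacting with a connected socket disconnects it, while interacting away from sockets destroys any pending cable.
; The same interaction also passes the player mesh to any overlapped machine's carry toggle.
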(event Custom|ToogleCableConection
  (params (TempActor :type Actor%20Object%20Reference))
  ;[0.7476 1 0.1815] Toogle the cable connections
  (if (not (Variables|/Game/SpaceFactory/Blueprints/CablesConector/BP_CableConectionSocket.BP_CableConectionSocket_C|GetisConnected (Variables|Cables|GetOverlapedSocket)))
    ;;[1 1 1] Cable execute conection
    (if (not (Variables|Cables|GetinConectionMode))
      ;;;[1 1 1] Start conection
      (Variables|Cables|SetinConectionMode true)
      (bind _output_get (Variables|Cables|SetCurrentConectionSocket (Variables|Cables|GetOverlapedSocket)))
      (Default|StartConnection _output_get TempActor)
      (else
        ;;;[1 1 1] Other end conection
        (Variables|Cables|SetinConectionMode false)
        (Class|CableComponent|SetAttachEndtoComponent (Variables|/Game/SpaceFactory/Blueprints/CablesConector/BP_Cable.BP_Cable_C|GetCable (Variables|/Game/SpaceFactory/Blueprints/CablesConector/BP_CableConectionSocket.BP_CableConectionSocket_C|GetConectionCable (Variables|Cables|GetCurrentConectionSocket))) (Variables|/Game/SpaceFactory/Blueprints/CablesConector/BP_CableConectionSocket.BP_CableConectionSocket_C|GetConnectionPoint (Variables|Cables|GetOverlapedSocket)) "None")
        ;;;[0 1 0.2258] Overlap conection make conection with the other end
        (Default|MakeConection (Variables|Cables|GetOverlapedSocket) (Variables|Cables|GetCurrentConectionSocket))
        ;;;[1 0.6557 0] Make the conection with the overlaped socket
        (Default|MakeConection (Variables|Cables|GetCurrentConectionSocket) (Variables|Cables|GetOverlapedSocket))))
    (else
      ;;[1 1 1] If is concted we disconect the cable
      (Default|DisconnectCable (Variables|Cables|GetOverlapedSocket))
      (CallFunction|StopCableConnection))))

(event Custom|StopCableConnection
  (bind _currentconectionsocket (Variables|Cables|GetCurrentConectionSocket))
  (bind _conectioncable (Variables|/Game/SpaceFactory/Blueprints/CablesConector/BP_CableConectionSocket.BP_CableConectionSocket_C|GetConectionCable _currentconectionsocket))
  ;[0.7476 1 0.1815] Toogle the cable connections
  ;;[1 1 1] Disable the conection
  (if (Variables|Cables|GetinConectionMode)
    (Variables|Cables|SetinConectionMode false)
    (Utilities|IsValid _currentconectionsocket
      (:Is%20Valid
        (Utilities|IsValid _conectioncable
          (:Is%20Valid
            (Actor|DestroyActor _conectioncable)))))))

(event Custom|ToogleCarryMachine
  (params (Parent :type Scene%20Component%20Object%20Reference))
  (bind _overlapingmachine (Variables|Default|GetOverlapingMachine))
  ;[1 1 1] Toogle Carrying machine
  (if (not (Variables|Default|GetisCarringMachine))
    (Utilities|IsValid _overlapingmachine
      (:Is%20Valid
        (Default|ToogleCarryMachine _overlapingmachine Parent)))))

(event Custom|ToogleMouse
  (params (PlayerController :type Player%20Controller%20Object%20Reference))
  ;[1 1 1] Enable or disable the mouse
  (if (Variables|Default|GetMouseMode)
    (Variables|Default|SetMouseMode false)
    (Variables|/Script/Engine.PlayerController|SetbShowMouseCursor PlayerController false)
    (Input|SetInputModeGameOnly PlayerController)
    (else
      (Variables|Default|SetMouseMode true)
      (Variables|/Script/Engine.PlayerController|SetbShowMouseCursor PlayerController true)
      (Input|SetInputModeGameandUI PlayerController 0 "DoNotLock" true))))

(event Custom|PlayerInteractObject
  (params (PlayerReference :type Character%20Object%20Reference))
  (bind _self self)
  (bind _self_2 self)
  ;[1 1 1] Player Interact with object
  (Utilities|FlowControl|Sequence
    (:then_0
      (Utilities|IsValid (Variables|BPC_SpaceFactory_C|GetOverlapedSocket self)
        (:Is%20Valid
          (CallFunction|ToogleCableConection _self_2 PlayerReference))
        (:Is%20Not%20Valid
          (CallFunction|StopCableConnection _self_2))))
    (:then_1
      ;;[1 1 1] Enable or disable the carry machine
      (Utilities|IsValid (Variables|BPC_SpaceFactory_C|GetOverlapingMachine _self)
        (:Is%20Valid
          (CallFunction|ToogleCarryMachine _self (Variables|/Script/Engine.Character|GetMesh PlayerReference)))))))

(event EventBeginPlay)

(event EventTick
  (params (DeltaSeconds :type Float%20%28single-precision%29)))